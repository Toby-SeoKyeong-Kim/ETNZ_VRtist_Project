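; Modular player character whose head, shirt and pants meshes and colors are customizable and loaded from a web server.
; Construction script slaves the parts to the body mesh via master pose.
; BeginPlay POSTs the player nickname, creates dynamic materials and shares most with MyGameInstance; JSON handlers apply each part's mesh and color, including headphones for one shirt type.
; CharacterHead and DrawonCanvas events also allow direct head swaps and recoloring.
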(event `self.CharacterHead`
  (params (Head_Index :type Integer))
  (bind _heads (`self.Heads`))
  (`SkinnedMeshComponent.SetSkinnedAssetAndUpdate` (`self.character_head`) (`|GetArrayItem` _heads (`KismetMathLibrary.Clamp` Head_Index 0 (`KismetArrayLibrary.Array_Length` _heads))) true))

(event `HTTPEvent`
  (params (JsonValue :type "SimpleJsonValue Object Reference") (Response :type "FetchResponse Object Reference"))
  (bind _returnvalue (`SimpleJsonValue.AsObject` JsonValue))
  (`self.BodyHTTP` (`SimpleJsonObject.GetObject` _returnvalue "body"))
  (`self.PantsHTTP` (`SimpleJsonObject.GetObject` _returnvalue "pants"))
  (`self.ShirtHTTP` (`SimpleJsonObject.GetObject` _returnvalue "shirt")))

(event `self.ReceiveBeginPlay`
  (`self.Material Init`))

(event `Draw on Canvas`
  (params (Color :type "LinearColor Structure") (Index :type Integer))
  (switch `int` Index
    (:`0`
      (`MaterialInstanceDynamic.SetVectorParameterValue` (`self.MaterialInstanceRef`) "color" Color)
      (`MaterialInstanceDynamic.SetVectorParameterValue` (`self.MaterialInstance2`) "color" Color))
    (:`1`
      (`MaterialInstanceDynamic.SetVectorParameterValue` (`self.ShirtMaterialRef`) "color" Color))
    (:`2`
      (`MaterialInstanceDynamic.SetVectorParameterValue` (`self.HeadPhoneMaterialRef`) "color" Color))
    (:`3`
      (`MaterialInstanceDynamic.SetVectorParameterValue` (`self.PantsMaterialRef`) "color" Color))))

(fn `BodyHTTP`
  (params (JSON :type "SimpleJsonObject Object Reference"))
  (bind _character_head (`self.character_head`))
  (bind _materialinstanceref (`self.MaterialInstanceRef`))
  (bind _materialinstance2 (`self.MaterialInstance2`))
  (bind _returnvalue (`KismetStringLibrary.Conv_StringToDouble` (`SimpleJsonObject.GetString` JSON "r")))
  (bind _returnvalue_2 (`KismetStringLibrary.Conv_StringToDouble` (`SimpleJsonObject.GetString` JSON "g")))
  (bind _returnvalue_3 (`KismetStringLibrary.Conv_StringToDouble` (`SimpleJsonObject.GetString` JSON "b")))
  (bind _returnvalue_4 (`KismetStringLibrary.Conv_StringToDouble` (`SimpleJsonObject.GetString` JSON "a")))
  (`SkinnedMeshComponent.SetSkinnedAssetAndUpdate` _character_head (`|GetArrayItem` (`self.Heads`) (`KismetStringLibrary.Conv_StringToInt` (`SimpleJsonObject.GetString` JSON "kind"))) true)
  (`MaterialInstanceDynamic.SetVectorParameterValue` _materialinstanceref "color" (make `LinearColor` _returnvalue _returnvalue_2 _returnvalue_3 _returnvalue_4))
  (`MaterialInstanceDynamic.SetVectorParameterValue` _materialinstance2 "color" (make `LinearColor` _returnvalue _returnvalue_2 _returnvalue_3 _returnvalue_4))
  (`PrimitiveComponent.SetMaterial` _character_head 0 _materialinstanceref)
  (`PrimitiveComponent.SetMaterial` (`self.Mesh`) 0 _materialinstance2))

(fn `Material Init`
  (bind _character_shirt (`self.character_shirt`))
  (bind _returnvalue (`FetchAPI.Fetch` "34.64.210.180:80/get" (make `FetchOptions` "POST" (`AdvancedIdentityLibrary.GetPlayerNickname` (`AdvancedSessionsLibrary.GetUniqueNetID` (`GameplayStatics.GetPlayerController` 0))))))
  (`FetchRequest.OnJson` _returnvalue (`|CreateDelegate` :!event `HTTPEvent`))
  (bind _returnvalue_2 (`KismetMaterialLibrary.CreateDynamicMaterialInstance` "/Game/Character/Material/PickerMaterial.PickerMaterial"))
  (set `self.MaterialInstanceRef` _returnvalue_2)
  (bind _returnvalue_3 (`KismetMaterialLibrary.CreateDynamicMaterialInstance` "/Game/Character/Material/PickerMaterial.PickerMaterial"))
  (set `self.MaterialInstance2` _returnvalue_3)
  (bind _returnvalue_4 (`KismetMaterialLibrary.CreateDynamicMaterialInstance` "/Game/Character/Material/PickerMaterialShirt.PickerMaterialShirt"))
  (set `self.ShirtMaterialRef` _returnvalue_4)
  (bind _returnvalue_5 (`KismetMaterialLibrary.CreateDynamicMaterialInstance` "/Game/Character/Material/PickerMaterialHeadPhone.PickerMaterialHeadPhone"))
  (set `self.HeadPhoneMaterialRef` _returnvalue_5)
  (bind _returnvalue_6 (`KismetMaterialLibrary.CreateDynamicMaterialInstance` "/Game/Character/Material/PickerMaterialPants.PickerMaterialPants"))
  (set `self.PantsMaterialRef` _returnvalue_6)
  (`PrimitiveComponent.SetMaterial` (`self.Mesh`) 0 (`self.MaterialInstance2`))
  (`PrimitiveComponent.SetMaterial` (`self.character_head`) 0 (`self.MaterialInstanceRef`))
  (`PrimitiveComponent.SetMaterial` _character_shirt 0 (`self.ShirtMaterialRef`))
  (`PrimitiveComponent.SetMaterial` _character_shirt 1 (`self.HeadPhoneMaterialRef`))
  (`PrimitiveComponent.SetMaterial` (`self.character_pants`) 0 (`self.PantsMaterialRef`))
  (bind _asmy_game_instance (cast `/Game/GameMode/MyGameInstance` (`GameplayStatics.GetGameInstance`)))
  (set `/Game/GameMode/MyGameInstance.HeadphoneRef` (`self.HeadPhoneMaterialRef`) _asmy_game_instance)
  (set `/Game/GameMode/MyGameInstance.MaterialRef` (`self.MaterialInstanceRef`) _asmy_game_instance)
  (set `/Game/GameMode/MyGameInstance.PantsRef` (`self.PantsMaterialRef`) _asmy_game_instance)
  (set `/Game/GameMode/MyGameInstance.ShirtRef` (`self.ShirtMaterialRef`) _asmy_game_instance))

(fn `PantsHTTP`
  (params (JSON :type "SimpleJsonObject Object Reference"))
  (bind _character_pants (`self.character_pants`))
  (bind _pantsmaterialref (`self.PantsMaterialRef`))
  (`SkinnedMeshComponent.SetSkinnedAssetAndUpdate` _character_pants (`|GetArrayItem` (`self.Pants`) (`KismetStringLibrary.Conv_StringToInt` (`SimpleJsonObject.GetString` JSON "kind"))) true)
  (`MaterialInstanceDynamic.SetVectorParameterValue` _pantsmaterialref "color" (make `LinearColor` (`KismetStringLibrary.Conv_StringToDouble` (`SimpleJsonObject.GetString` JSON "r")) (`KismetStringLibrary.Conv_StringToDouble` (`SimpleJsonObject.GetString` JSON "g")) (`KismetStringLibrary.Conv_StringToDouble` (`SimpleJsonObject.GetString` JSON "b")) (`KismetStringLibrary.Conv_StringToDouble` (`SimpleJsonObject.GetString` JSON "a"))))
  (`PrimitiveComponent.SetMaterial` _character_pants 0 _pantsmaterialref))

(fn `ShirtHTTP`
  (params (JSON :type "SimpleJsonObject Object Reference"))
  (bind _character_shirt (`self.character_shirt`))
  (bind _shirtmaterialref (`self.ShirtMaterialRef`))
  (bind _headphonematerialref (`self.HeadPhoneMaterialRef`))
  (bind _returnvalue (`KismetStringLibrary.Conv_StringToInt` (`SimpleJsonObject.GetString` JSON "kind")))
  (`SkinnedMeshComponent.SetSkinnedAssetAndUpdate` _character_shirt (`|GetArrayItem` (`self.Shirts`) _returnvalue) true)
  (`MaterialInstanceDynamic.SetVectorParameterValue` _shirtmaterialref "color" (make `LinearColor` (`KismetStringLibrary.Conv_StringToDouble` (`SimpleJsonObject.GetString` JSON "r")) (`KismetStringLibrary.Conv_StringToDouble` (`SimpleJsonObject.GetString` JSON "g")) (`KismetStringLibrary.Conv_StringToDouble` (`SimpleJsonObject.GetString` JSON "b")) (`KismetStringLibrary.Conv_StringToDouble` (`SimpleJsonObject.GetString` JSON "a"))))
  (`PrimitiveComponent.SetMaterial` _character_shirt 0 _shirtmaterialref)
  (if (== _returnvalue 1)
    (`MaterialInstanceDynamic.SetVectorParameterValue` _headphonematerialref "color" (make `LinearColor` (`KismetStringLibrary.Conv_StringToDouble` (`SimpleJsonObject.GetString` JSON "hr")) (`KismetStringLibrary.Conv_StringToDouble` (`SimpleJsonObject.GetString` JSON "hg")) (`KismetStringLibrary.Conv_StringToDouble` (`SimpleJsonObject.GetString` JSON "hb")) (`KismetStringLibrary.Conv_StringToDouble` (`SimpleJsonObject.GetString` JSON "ha"))))
    (`PrimitiveComponent.SetMaterial` (`self.character_shirt`) 1 _headphonematerialref)))

(fn `UserConstructionScript`
  (`SkinnedMeshComponent.SetLeaderPoseComponent` (`self.character_head`) (`self.Mesh`) false)
  (`SkinnedMeshComponent.SetLeaderPoseComponent` (`self.character_shirt`) (`self.Mesh`) false)
  (`SkinnedMeshComponent.SetLeaderPoseComponent` (`self.character_pants`) (`self.Mesh`) false))