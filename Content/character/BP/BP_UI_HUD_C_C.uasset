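; BP_UI_HUD_C_C is a UI Blueprint for character customization that relays head changes to a character.
; Its CharacterHead event passes a head index to the stored Character reference through CharacterHeadMessage.
; Logic to find that character by BP_UI_C_C_interface and show the WDG_Character widget is disconnected from the empty BeginPlay, so it never runs.
; Nothing else here assigns the Character reference.
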(event `self.ReceiveBeginPlay`
  ;[1 1 1] 캐릭터 변경 적용 위젯
)

(event `self.CharacterHead`
  (params (Head_Index :type Integer))
  ;[1 1 1] 캐릭터 변경 적용 메세지
  (message `/Game/Character/BP/BP_UI_C_C_interface.CharacterHead` (`self.Character`) Head_Index))

(fn `UserConstructionScript`)