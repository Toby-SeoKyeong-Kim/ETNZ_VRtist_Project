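; VR player pawn for the menu and character customization, with world-space host, join, character and color picker panels.
; OpenWindows parks all panels far below, then teleports the chosen one into view, starting a server search for Join.
; Right grip applies the hand's selected color to the game-instance material chosen by the character widget.
; Left grip toggles the left hand's drawing flag, and axis inputs scroll widgets through each hand.
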(event `self.ReceiveBeginPlay`
  (`self.OpenWindows` 0)
  (bind _returnvalue (`GameplayStatics.GetCurrentLevelName` true))
  (if (== _returnvalue "Character")
    (bind _asmaster_widget (cast `/Game/Widgets/MasterWidget` (`WidgetComponent.GetWidget` (`self.MasterWidget`))))
    (set `/Game/Widgets/MasterWidget.CharacterRef` self _asmaster_widget)
    (else
      (`self.IsPicker` true))))

(event `InputAction|GripL`
  (params (Key :type "Key Structure"))
  (bind _lefthand (`self.LeftHand`))
  (:`Pressed`
    (set `HandController.IsDrawingCpp` true _lefthand))
  (:`Released`
    (set `HandController.IsDrawingCpp` false _lefthand)))

(event `InputAction|GripR`
  (params (Key :type "Key Structure"))
  (:`Pressed`
    (bind _asbp_hand_controller_2 (cast `/Game/BP/BP_HandController2` (`self.RightHand`)))
    (bind _ascharacter_widget (cast `/Game/Widgets/CharacterWidget` (`WidgetComponent.GetWidget` (`self.Character`))))
    (bind _asmy_game_instance (cast `/Game/GameMode/MyGameInstance` (`GameplayStatics.GetGameInstance`)))
    (switch `int` (`/Game/Widgets/CharacterWidget.KindIndex` _ascharacter_widget)
      (:`0`
        (bind _selectedcolor (`/Game/BP/BP_HandController2.SelectedColor` _asbp_hand_controller_2))
        (`MaterialInstanceDynamic.SetVectorParameterValue` (`/Game/GameMode/MyGameInstance.MaterialRef` _asmy_game_instance) "color" _selectedcolor))
      (:`1`
        (`MaterialInstanceDynamic.SetVectorParameterValue` (`/Game/GameMode/MyGameInstance.ShirtRef` _asmy_game_instance) "color" _selectedcolor))
      (:`2`
        (`MaterialInstanceDynamic.SetVectorParameterValue` (`/Game/GameMode/MyGameInstance.PantsRef` _asmy_game_instance) "color" _selectedcolor))
      (:`3`
        (`MaterialInstanceDynamic.SetVectorParameterValue` (`/Game/GameMode/MyGameInstance.HeadphoneRef` _asmy_game_instance) "color" _selectedcolor)))))

(event `InputAxis|MouseWheelL`
  (params (AxisValue :type "Float (single-precision)"))
  (bind _asbp_hand_controller_2 (cast `/Game/BP/BP_HandController2` (`self.LeftHand`)))
  (`WidgetInteractionComponent.ScrollWheel` (`HandController.Widgetinteraction` _asbp_hand_controller_2) (* AxisValue -1.0)))

(event `InputAxis|MouseWheelR`
  (params (AxisValue :type "Float (single-precision)"))
  (bind _asbp_hand_controller_2 (cast `/Game/BP/BP_HandController2` (`self.RightHand`)))
  (`WidgetInteractionComponent.ScrollWheel` (`HandController.Widgetinteraction` _asbp_hand_controller_2) (* AxisValue -1.0)))

(fn `OpenWindows`
  (params (index :type Integer))
  (bind _joinwidget (`self.JoinWidget`))
  (`SceneComponent.K2_SetRelativeLocation` (`self.Character`) (0.0 0.0 -900.0) false true)
  (`SceneComponent.K2_SetRelativeLocation` (`self.ColorPickerBP`) (0.0 0.0 -900.0) false false)
  (`SceneComponent.K2_SetRelativeLocation` (`self.HostWidget`) (0.0 0.0 -900.0) false false)
  (`SceneComponent.K2_SetRelativeLocation` (`self.JoinWidget`) (0.0 0.0 -900.0) false false)
  (switch `int` index
    (:`1`
      (`SceneComponent.K2_SetRelativeLocation` (`self.HostWidget`) (202.0 70.0 40.0) false true))
    (:`2`
      (`SceneComponent.K2_SetRelativeLocation` _joinwidget (202.0 70.0 40.0) false true)
      (bind _asjoin_widget (cast `/Game/Widgets/JoinWidget` (`WidgetComponent.GetWidget` _joinwidget)))
      (`/Game/Widgets/JoinWidget.SearchSevers` _asjoin_widget))
    (:`3`
      (`SceneComponent.K2_SetRelativeLocation` (`self.Character`) (206.0 70.0 15.0) false true)
      (`SceneComponent.K2_SetRelativeLocation` (`self.ColorPickerBP`) (202.0 80.0 6.0) false true))))

(fn `UserConstructionScript`)