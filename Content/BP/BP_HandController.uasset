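; Hand controller for a music game that turns touches on drum sequencer and keyboard components into actions, with its mesh material taken from the game instance.
; Interaction-area overlaps dispatch by component tag to toggle the sequencer clock or flag per-hand block editing on DJController, parsing block index from the name's last digit.
; Keys set per-hand pitch from key index and octave, then trigger an attack.
; Key release and EQ bar handlers are unused stubs.
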(event `self.ReceiveBeginPlay`
  (bind _asmy_game_instance (cast `/Game/GameMode/MyGameInstance` (`GameplayStatics.GetGameInstance`)))
  (`PrimitiveComponent.SetMaterial` (`self.handmesh`) 0 (`/Game/GameMode/MyGameInstance.MaterialRef` _asmy_game_instance)))

(event `self.InteractionArea.OnComponentBeginOverlap`
  (params (OverlappedComponent :type "PrimitiveComponent Object Reference") (OtherActor :type "Actor Object Reference") (OtherComp :type "PrimitiveComponent Object Reference") (OtherBodyIndex :type Integer) (bFromSweep :type Boolean) (SweepResult :type "HitResult Structure (by ref)"))
  (`self.SequenceBlockEventHandle` OtherComp)
  (`self.PlaySequencerHandle` OtherComp)
  (`self.KeyAttackHandle` OtherComp))

(event `self.InteractionArea.OnComponentEndOverlap`
  (params (OverlappedComponent :type "PrimitiveComponent Object Reference") (OtherActor :type "Actor Object Reference") (OtherComp :type "PrimitiveComponent Object Reference") (OtherBodyIndex :type Integer))
  (`self.SequenceBlockReleaseHandle` OtherComp))

(fn `EQBarHandle`
  (params (Other :type "PrimitiveComponent Object Reference"))
  (if (`ActorComponent.ComponentHasTag` Other "EQBar")
    _))

(fn `KeyAttackHandle`
  (params (OtherComp :type "PrimitiveComponent Object Reference"))
  (if (`ActorComponent.ComponentHasTag` OtherComp "Keys")
    (bind _askey_board_bp (cast `/Game/BP/KeyBoardBP` (`ActorComponent.GetOwner` OtherComp)))
    (bind _asstatic_mesh_component (cast `StaticMeshComponent` OtherComp))
    (bind _returnvalue (`self.GetHandSide`))
    (switch `EControllerHand` _returnvalue
      (:`Left`
        (bind _returnvalue_2 (`AudioComponent.GetParameterInterface` (`/Game/BP/KeyBoardBP.KeyBoardEngine` _askey_board_bp)))
        (bind _returnvalue_3 (+ (`KismetArrayLibrary.Array_Find` (`/Game/BP/KeyBoardBP.Keys` _askey_board_bp) _asstatic_mesh_component) (* (`/Game/BP/KeyBoardBP.Octave` _askey_board_bp) 12)))
        (`AudioParameterInterface.SetFloat` _returnvalue_2 "SineFrequency01" (`KismetMathLibrary.Conv_IntToDouble` _returnvalue_3))
        (`AudioParameterInterface.Trigger` _returnvalue_2 "Attack"))
      (:`Right`
        (`AudioParameterInterface.SetFloat` _returnvalue_2 "SineFrequency02" (`KismetMathLibrary.Conv_IntToDouble` _returnvalue_3))
        (`AudioParameterInterface.Trigger` _returnvalue_2 "Attack2")))))

(fn `KeyReleaseHandle`
  (params (OtherComp :type "PrimitiveComponent Object Reference")))

(fn `PlaySequencerHandle`
  (params (OtherActor :type "PrimitiveComponent Object Reference"))
  (if (`ActorComponent.ComponentHasTag` OtherActor "PlaySequencer")
    (bind _asdrum_sequencer (cast `/Game/BP/DrumSequencer` (`ActorComponent.GetOwner` OtherActor)))
    (bind _sequencerclock (`/Game/BP/DrumSequencer.SequencerClock` _asdrum_sequencer))
    (bind _returnvalue (`QuartzClockHandle.IsClockRunning` _sequencerclock))
    (if _returnvalue
      (`QuartzClockHandle.StopClock` _sequencerclock false)
      (else
        (`QuartzClockHandle.ResumeClock` _sequencerclock)))))

(fn `SequenceBlockEventHandle`
  (params (OtherComp :type "PrimitiveComponent Object Reference"))
  (bind _returnvalue (`KismetSystemLibrary.GetObjectName` OtherComp))
  (bind _returnvalue_2 (`ActorComponent.GetOwner` OtherComp))
  (bind _returnvalue_3 (`KismetStringLibrary.Conv_StringToInt` (`KismetStringLibrary.GetSubstring` _returnvalue (- (`KismetStringLibrary.Len` _returnvalue) 1))))
  (if (`ActorComponent.ComponentHasTag` OtherComp "SequenceBlock")
    (bind _returnvalue_4 (`self.GetHandSide`))
    (switch `EControllerHand` _returnvalue_4
      (:`Left`
        (bind _returnvalue_5 (`GameplayStatics.GetActorOfClass` "/Game/BP/DJController.DJController_C"))
        (set `/Game/BP/DJController.LeftEditingBlock` true _returnvalue_5)
        (set `/Game/BP/DJController.LeftEditingIndex` _returnvalue_3 _returnvalue_5)
        (bind _asdrum_sequencer (cast `/Game/BP/DrumSequencer` _returnvalue_2))
        (set `/Game/BP/DJController.DrumSequencerRef` _asdrum_sequencer _returnvalue_5))
      (:`Right`
        (bind _returnvalue_6 (`GameplayStatics.GetActorOfClass` "/Game/BP/DJController.DJController_C"))
        (set `/Game/BP/DJController.RightEditingBlock` true _returnvalue_6)
        (set `/Game/BP/DJController.RightEditingIndex` _returnvalue_3 _returnvalue_6)
        (bind _asdrum_sequencer_2 (cast `/Game/BP/DrumSequencer` _returnvalue_2))
        (set `/Game/BP/DJController.DrumSequencerRef` _asdrum_sequencer_2 _returnvalue_6)))))

(fn `SequenceBlockReleaseHandle`
  (params (self2 :type "ActorComponent Object Reference"))
  (if (`ActorComponent.ComponentHasTag` self2 "SequenceBlock")
    (bind _returnvalue (`self.GetHandSide`))
    (switch `EControllerHand` _returnvalue
      (:`Left`
        (bind _returnvalue_2 (`GameplayStatics.GetActorOfClass` "/Game/BP/DJController.DJController_C"))
        (set `/Game/BP/DJController.LeftEditingBlock` false _returnvalue_2))
      (:`Right`
        (bind _returnvalue_3 (`GameplayStatics.GetActorOfClass` "/Game/BP/DJController.DJController_C"))
        (set `/Game/BP/DJController.RightEditingBlock` false _returnvalue_3)))))

(fn `UserConstructionScript`)