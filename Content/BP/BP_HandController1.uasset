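; BP_HandController1 is a VR hand actor attached to the player character, handling multiplayer ladder climbing.
; Overlapping "ladders"-tagged components sets CanClimb and plays haptics on the name-matched player controller.
; Gripping anchors the hand and cancels the other's climb; authority Tick moves the parent opposite hand displacement, passing its transform to ClimbRep.
; SequenceBlockEventHandle flags left-hand block editing on the DJController for "SequenceBlock"-tagged components.
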(event `self.ReceiveBeginPlay`)

(event `self.handmesh.OnComponentBeginOverlap`
  (params (OverlappedComponent :type "PrimitiveComponent Object Reference") (OtherActor :type "Actor Object Reference") (OtherComp :type "PrimitiveComponent Object Reference") (OtherBodyIndex :type Integer) (bFromSweep :type Boolean) (SweepResult :type "HitResult Structure (by ref)"))
  (if (`ActorComponent.ComponentHasTag` OtherComp "ladders")
    (set `self.canClimb` true)
    (bind _asbp_vrcharacter_2 (cast `/Game/BP/BP_VRCharacter2` (`self.GetAttachParentActor`)))
    (bind _asmy_game_mode (cast `/Game/GameMode/MyGameMode` (`GameplayStatics.GetGameMode`)))
    (for _array_element (`/Game/GameMode/MyGameMode.allPCs` _asmy_game_mode)
      (if (== (`/Game/BP/BP_VRCharacter2.Name` _asbp_vrcharacter_2) (`AdvancedSessionsLibrary.GetPlayerName` _array_element))
        (bind _returnvalue (`self.GetHandSide`))
        (`PlayerController.PlayHapticEffect` _array_element "/Game/BP/MotionControllerHaptics.MotionControllerHaptics" _returnvalue 1.0 false)
        (break)))))

(event `self.handmesh.OnComponentEndOverlap`
  (params (OverlappedComponent :type "PrimitiveComponent Object Reference") (OtherActor :type "Actor Object Reference") (OtherComp :type "PrimitiveComponent Object Reference") (OtherBodyIndex :type Integer))
  (if (`ActorComponent.ComponentHasTag` OtherComp "ladders")
    (set `self.canClimb` false)))

(event `GripHandle`
  (set `self.isClimbing` true)
  (set `self.ClimbingStartLocation` (`self.K2_GetActorLocation`))
  (bind _asbp_hand_controller_1 (cast `/Game/BP/BP_HandController1` (`self.GetOtherHand`)))
  (set `/Game/BP/BP_HandController1.isClimbing` false _asbp_hand_controller_1))

(event `ReleaseHandle`
  (set `self.isClimbing` false))

(event `self.ReceiveTick`
  (params (DeltaSeconds :type "Float (single-precision)"))
  (bind _returnvalue (`self.GetAttachParentActor`))
  (if (`self.isClimbing`)
    (`/Engine/EditorBlueprintResources/ActorMacros.Switch Has Authority`
      (:`Authority`
        (`self.K2_AddActorWorldOffset` _returnvalue (* (- (`self.K2_GetActorLocation`) (`self.ClimbingStartLocation`)) -1.0) false false)
        (`self.climbRep` (`self.GetTransform` _returnvalue))))))

(event `climbRep`
  (params (NewTransform :type "Transform Structure"))
  (`self.K2_SetActorTransform` (`self.GetAttachParentActor`) NewTransform false false))

(fn `SequenceBlockEventHandle`
  (params (OtherComp :type "PrimitiveComponent Object Reference"))
  (if (`ActorComponent.ComponentHasTag` OtherComp "SequenceBlock")
    (bind _returnvalue (`self.GetHandSide`))
    (switch `EControllerHand` _returnvalue
      (:`Left`
        (bind _returnvalue_2 (`GameplayStatics.GetActorOfClass` "/Game/BP/DJController.DJController_C"))
        (set `/Game/BP/DJController.LeftEditingBlock` true _returnvalue_2)))))

(fn `UserConstructionScript`)