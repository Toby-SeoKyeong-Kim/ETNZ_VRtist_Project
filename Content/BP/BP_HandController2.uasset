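; VR hand controller that lets the right hand point at a color picker to choose a character color.
; Each tick it line-traces from the motion controller and moves a marker onto components tagged HueCon or SVCon.
; The hit's local position gives hue by angle, or saturation and value by mapped axes.
; UpdateSelectedColor stores the color and tints the marker, SV panel and BP_CharacterPicker2's widget preview.
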(event `self.ReceiveBeginPlay`
  (`SceneComponent.SetVisibility` (`self.Marker`) false false)
  (bind _returnvalue (`PrimitiveComponent.CreateDynamicMaterialInstance` (`self.Marker`) 0 "/Game/Character/Material/PickerMaterial.PickerMaterial" "None"))
  (set `self.MarkerMat` _returnvalue)
  (bind _returnvalue_2 (`GameplayStatics.GetActorOfClass` "/Game/BP/BP_CharacterPicker2.BP_CharacterPicker2_C"))
  (set `self.PicerRef` _returnvalue_2))

(event `self.ReceiveTick`
  (params (DeltaSeconds :type "Float (single-precision)"))
  (bind _motioncontroller (`self.MotionController`))
  (bind _marker (`self.Marker`))
  (bind _returnvalue (`SceneComponent.K2_GetComponentLocation` _motioncontroller))
  (bind _returnvalue_2 (`self.GetHandSide`))
  (switch `EControllerHand` _returnvalue_2
    (:`Right`
      (bind (_outhit _returnvalue_3) (`KismetSystemLibrary.LineTraceSingle` :`Start` _returnvalue :`End` (+ _returnvalue (* (`SceneComponent.GetForwardVector` _motioncontroller) 700.0)) :`TraceChannel` "TraceTypeQuery2" :`bTraceComplex` true :`DrawTime` 0.1))
      (if _returnvalue_3
        (bind (_bblockinghit _binitialoverlap _time _distance _location _impactpoint _normal _impactnormal _physmat _hitactor _hitcomponent) (`GameplayStatics.BreakHitResult` _outhit))
        (if (`ActorComponent.ComponentHasTag` _hitcomponent "HueCon")
          (set `self.IsHovering` true)
          (`SceneComponent.SetVisibility` _marker true false)
          (`SceneComponent.K2_SetWorldLocation` _marker _location false true)
          (bind (_returnvalue_x _returnvalue_y _returnvalue_z) (`KismetMathLibrary.BreakVector` (`KismetMathLibrary.InverseTransformLocation` (`SceneComponent.K2_GetComponentToWorld` _hitcomponent) _location)))
          (bind _returnvalue_4 (`KismetMathLibrary.DegAtan2` _returnvalue_x _returnvalue_z))
          (if (< _returnvalue_4 0.0)
            (set `self.Hue` (- 360.0 (+ (- 180.0 (`KismetMathLibrary.Abs` _returnvalue_4)) 180.0)))
            (else
              (set `self.Hue` (- 360.0 _returnvalue_4))))
          (bind _returnvalue_5 (`ActorComponent.GetOwner` _hitcomponent))
          (`self.UpdateSelectedColor` _returnvalue_5)
          (elif (`ActorComponent.ComponentHasTag` _hitcomponent "SVCon")
            (set `self.IsHovering` true)
            (`SceneComponent.SetVisibility` _marker true false)
            (`SceneComponent.K2_SetWorldLocation` _marker _location false true)
            (bind (_returnvalue_x_2 _returnvalue_y_2) (`KismetMathLibrary.BreakVector` (`KismetMathLibrary.InverseTransformLocation` (`SceneComponent.K2_GetComponentToWorld` _hitcomponent) _location)))
            (set `self.Saturation` (`KismetMathLibrary.MapRangeClamped` _returnvalue_y_2 -45.0 45.0 0.0 1.0))
            (set `self.Value` (`KismetMathLibrary.MapRangeClamped` _returnvalue_x_2 -45.0 45.0 1.0))
            (`self.UpdateSelectedColor` _returnvalue_5 true)
            (else
              (`SceneComponent.SetVisibility` (`self.Marker`) false false :!label _label)
              (set `self.IsHovering` false))))
        (else
          (goto _label))))))

(fn `HueConFunc`)

(fn `SVConFunc`)

(fn `UpdateSelectedColor`
  (params (Actor :type "Actor Object Reference") (IsSV :type Boolean))
  (bind _hue (`self.Hue`))
  (bind _markermat (`self.MarkerMat`))
  (bind _returnvalue (`KismetMathLibrary.HSVToRGB` _hue (`self.Saturation`) (`self.Value`)))
  (bind _returnvalue_2 (`KismetMathLibrary.HSVToRGB` _hue 1.0 1.0))
  (bind _returnvalue_3 (`WidgetComponent.GetWidget` (`/Game/BP/BP_CharacterPicker2.Character` (`self.PicerRef`))))
  (if IsSV
    (`MaterialInstanceDynamic.SetVectorParameterValue` _markermat "color" _returnvalue)
    (set `self.SelectedColor` _returnvalue)
    (bind _ascharacter_widget (cast `/Game/Widgets/CharacterWidget` _returnvalue_3))
    (`Border.SetBrushColor` (`/Game/Widgets/CharacterWidget.ColorPrev` _ascharacter_widget) _returnvalue)
    (else
      (`MaterialInstanceDynamic.SetVectorParameterValue` _markermat "color" _returnvalue_2)
      (bind _ascolor_picker_bp (cast `/Game/BP/ColorPickerBP` Actor))
      (`MaterialInstanceDynamic.SetVectorParameterValue` (`/Game/BP/ColorPickerBP.SvConMat` _ascolor_picker_bp) "color" _returnvalue_2)
      (set `self.SelectedColor` _returnvalue_2)
      (bind _ascharacter_widget_2 (cast `/Game/Widgets/CharacterWidget` _returnvalue_3))
      (`Border.SetBrushColor` (`/Game/Widgets/CharacterWidget.ColorPrev` _ascharacter_widget_2) _returnvalue_2))))

(fn `UserConstructionScript`)