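; Left play button actor whose mesh shows pressed state through a glow and a short vertical move.
; BeginPlay lights the mesh via a dynamic material's "Light" parameter and lowers it with MoveComponentTo.
; Collision overlaps only toggle IsPressed on begin; ending turns the glow off.
; IsPressed clears before its end-overlap check, so the raise branch never runs; a HandController cast is unwired.
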(event `self.ReceiveBeginPlay`
  (bind _button_button1 (`self.Button_Button1`))
  (bind _button_button1_2 (`self.Button_Button1`))
  (bind (_returnvalue_location _returnvalue_rotation) (`KismetMathLibrary.BreakTransform` (`SceneComponent.GetRelativeTransform` _button_button1)))
  ;[1 1 1] 빛나는 머테리얼
  (bind _returnvalue (`PrimitiveComponent.CreateDynamicMaterialInstance` _button_button1_2 0 (`PrimitiveComponent.GetMaterial` _button_button1_2 0) "None"))
  (`MaterialInstanceDynamic.SetScalarParameterValue` _returnvalue "Light" 20.0)
  ;[1 1 1] 버튼 눌리는 애니메이션
  (`KismetSystemLibrary.MoveComponentTo` _button_button1 (- _returnvalue_location (0.0 0.0 3.0)) _returnvalue_rotation true false 0.5))

(event `self.collision.OnComponentBeginOverlap`
  (params (OverlappedComponent :type "PrimitiveComponent Object Reference") (OtherActor :type "Actor Object Reference") (OtherComp :type "PrimitiveComponent Object Reference") (OtherBodyIndex :type Integer) (bFromSweep :type Boolean) (SweepResult :type "HitResult Structure (by ref)"))
  ;[1 1 1] 버튼 눌린 콜리전
  (set `self.Is pressed` true))

(event `self.collision.OnComponentEndOverlap`
  (params (OverlappedComponent :type "PrimitiveComponent Object Reference") (OtherActor :type "Actor Object Reference") (OtherComp :type "PrimitiveComponent Object Reference") (OtherBodyIndex :type Integer))
  (bind _button_button1 (`self.Button_Button1`))
  (bind _button_button1_2 (`self.Button_Button1`))
  (bind _button_button1_3 (`self.Button_Button1`))
  (bind _button_button1_4 (`self.Button_Button1`))
  (bind (_returnvalue_location _returnvalue_rotation) (`KismetMathLibrary.BreakTransform` (`SceneComponent.GetRelativeTransform` _button_button1)))
  (bind (_returnvalue_location_2 _returnvalue_rotation_2) (`KismetMathLibrary.BreakTransform` (`SceneComponent.GetRelativeTransform` _button_button1_2)))
  ;[1 1 1] 버튼 뗀 콜리전
  (set `self.Is pressed` false)
  (if (`self.Is pressed`)
    ;[1 1 1] 이미 버튼이 눌렸었을 땐 +0.5
    ;;[1 1 1] 빛꺼지는 머테리얼
    (bind _returnvalue (`PrimitiveComponent.CreateDynamicMaterialInstance` _button_button1_3 0 (`PrimitiveComponent.GetMaterial` _button_button1_3 0) "None"))
    (`MaterialInstanceDynamic.SetScalarParameterValue` _returnvalue "Light" 0.0)
    ;;[1 1 1] 버튼 뗀 애니메이션
    (`KismetSystemLibrary.MoveComponentTo` _button_button1_2 (+ _returnvalue_location_2 (0.0 0.0 3.0)) _returnvalue_rotation_2 false false 1.0)
    (else
      ;[1 1 1] 버튼이 눌리지 않았던 상태에선 0
      ;;[1 1 1] 빛꺼지는 머테리얼
      (bind _returnvalue_2 (`PrimitiveComponent.CreateDynamicMaterialInstance` _button_button1_4 0 (`PrimitiveComponent.GetMaterial` _button_button1_4 0) "None"))
      (`MaterialInstanceDynamic.SetScalarParameterValue` _returnvalue_2 "Light" 0.0)
      ;;[1 1 1] 버튼 뗀 애니메이션
      (`KismetSystemLibrary.MoveComponentTo` _button_button1 (+ _returnvalue_location (0.0 0.0 0.0)) _returnvalue_rotation false false 1.0)
      (set `self.Is pressed` false))))

(fn `UserConstructionScript`)