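; BP_VRCharacter is the player character, which walks around and can hand control over to a DJController.
; Movement axes follow the camera's forward and right vectors, and TurnPad yaw input is eased with FInterpTo.
; When Controllable, pressing E finds ready DJController actors, flags them as controlled by this character and possesses them, hiding the character and showing the controller.
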(event `InputAxis|TurnPad`
  (params (AxisValue :type "Float (single-precision)"))
  (bind _output_get (set `self.CurrentYawInput` (`KismetMathLibrary.FInterpTo` (`self.CurrentYawInput`) AxisValue (`GameplayStatics.GetWorldDeltaSeconds`) 0.5)))
  (`self.AddControllerYawInput` _output_get))

(event `InputAxis|MoveForward`
  (params (AxisValue :type "Float (single-precision)"))
  (`self.AddMovementInput` (`self.GetActorForwardVector` (`GameplayStatics.GetPlayerCameraManager` 0)) AxisValue))

(event `InputAxis|MoveRight`
  (params (AxisValue :type "Float (single-precision)"))
  (`self.AddMovementInput` (`self.GetActorRightVector` (`GameplayStatics.GetPlayerCameraManager` 0)) AxisValue))

(event `Key|E`
  (params (Key :type "Key Structure"))
  (:`Pressed`
    (if (`self.Controllable`)
      (bind _outactors (`GameplayStatics.GetAllActorsOfClass` "/Game/BP/DJController.DJController_C"))
      (for _array_element _outactors
        (if (`/Game/BP/DJController.IsReady` _array_element)
          (set `/Game/BP/DJController.Controlling` true _array_element)
          (set `/Game/BP/DJController.ControlleringCharacter` self _array_element)
          (`Controller.Possess` (`GameplayStatics.GetPlayerController` 0) _array_element)
          (`self.ToggleHidden` true)
          (`self.ToggleHidden` _array_element false))))))

(fn `UserConstructionScript`)