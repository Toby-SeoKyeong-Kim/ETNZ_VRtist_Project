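; BP_DiscoLight05 is a disco strobe light that blinks a spotlight along with the glow of its mesh.
; BeginPlay creates a dynamic material instance on the static mesh.
; Tick feeds a Delay of BlinkTime, which paces each toggle of spotlight visibility.
; A FlipFlop after the toggle alternates the material's EmissionPower parameter between zero and the EmissionPower variable.
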(event `self.ReceiveTick`
  (params (DeltaSeconds :type "Float (single-precision)"))
  ;[1 1 1] Strobe light graph controls the frequency of blinking light
  (`KismetSystemLibrary.Delay` (`self.BlinkTime`))
  (`SceneComponent.ToggleVisibility` (`self.SpotLight`) false)
  (bind _isa (`/Engine/EditorBlueprintResources/StandardMacros.FlipFlop`)
    (:`A`
      _)
    (:`B`
      _))
  (`MaterialInstanceDynamic.SetScalarParameterValue` (`self.DynamicInstance`) "EmissionPower" (`KismetMathLibrary.SelectFloat` 0.0 (`self.EmissionPower`) _isa)))

(event `self.ReceiveBeginPlay`
  ;[1 1 1] Strobe light graph controls the frequency of blinking light
  (bind _returnvalue (`PrimitiveComponent.CreateDynamicMaterialInstance` (`self.StaticMeshComponent01`) 0 null "None"))
  (set `self.DynamicInstance` _returnvalue))

(fn `UserConstructionScript`)